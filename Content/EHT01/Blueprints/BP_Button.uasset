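; BP_Button is an interactable button that removes the level's BP_Door and itself when the player presses PrimaryAction nearby.
; On BeginPlay it caches the door found through GetActorOfClass.
; Box overlaps with BP_FirstPersonCharacter toggle the character's AllowInteraction flag, the button's input and a TextRender prompt.
; Enabling input only while overlapping gates the press, which destroys both actors.
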(event OnComponentBeginOverlap(Box)
  (params (OverlappedComponent :type Primitive%20Component%20Object%20Reference) (OtherActor :type Actor%20Object%20Reference) (OtherComp :type Primitive%20Component%20Object%20Reference) (OtherBodyIndex :type Integer) (bFromSweep :type Boolean) (SweepResult :type Hit%20Result%20Structure%20%28by%20ref%29))
  (bind _asbp_first_person_character (Utilities|Casting|CastToBP_FirstPersonCharacter OtherActor))
  (Variables|/Game/EHT01/Blueprints/BP_FirstPersonCharacter.BP_FirstPersonCharacter_C|SetallowInteraction _asbp_first_person_character true)
  (Input|EnableInput (Game|GetPlayerController 0))
  (Rendering|SetVisibility (Variables|Default|GetTextRender) true false))

(event OnComponentEndOverlap(Box)
  (params (OverlappedComponent :type Primitive%20Component%20Object%20Reference) (OtherActor :type Actor%20Object%20Reference) (OtherComp :type Primitive%20Component%20Object%20Reference) (OtherBodyIndex :type Integer))
  (bind _asbp_first_person_character (Utilities|Casting|CastToBP_FirstPersonCharacter OtherActor))
  (Variables|/Game/EHT01/Blueprints/BP_FirstPersonCharacter.BP_FirstPersonCharacter_C|SetallowInteraction _asbp_first_person_character false)
  (Input|DisableInput (Game|GetPlayerController 0))
  (Rendering|SetVisibility (Variables|Default|GetTextRender) false false))

(event EventBeginPlay
  (bind _returnvalue (Actor|GetActorOfClass "/Game/EHT01/Blueprints/BP_Door.BP_Door_C"))
  (Variables|Default|SetDoor _returnvalue))

(event Input|ActionEvents|InputActionPrimaryAction
  (params (Key :type Key%20Structure :default "None"))
  (:Pressed
    (Actor|DestroyActor (Variables|Default|GetDoor))
    (Actor|DestroyActor)))

(fn ConstructionScript)