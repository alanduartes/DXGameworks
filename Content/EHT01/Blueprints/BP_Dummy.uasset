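; BP_Dummy is an enemy target that patrols sideways along world Y, shoots at the player and is destroyed when damage depletes its health.
; BeginPlay randomizes speed and patrol distance; Move drives movement velocity directly, reversing after that distance from the last turning point.
; Each tick, a debug-drawn box trace toward its Box component looks for BP_FirstPersonCharacter.
; On a hit, it fires a BP_Projectile aimed at the player, rate-limited by a timer.
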(event EventBeginPlay
  (Variables|Default|SetRandom%20Distance (Math|Random|RandomFloatinRange (Variables|Default|GetminRangeDistance) (Variables|Default|GetmaxRangeDistance)))
  (Variables|Default|SetVelocity%20Y (Math|Random|RandomFloatinRange (Variables|Default|GetminVelocity) (Variables|Default|GetmaxVelocity))))

(event EventTick
  (params (DeltaSeconds :type Float%20%28single-precision%29))
  (Variables|Default|SetTime%20to%20Shoot (+ DeltaSeconds (Variables|Default|GetTime%20to%20Shoot)))
  (CallFunction|LookingforPlayer)
  (if (Variables|Default|GetisStoped)
    (Variables|Default|SetStartDistance (Transformation|GetActorTransform))
    (Variables|Default|SetisStoped false)
    (else
      (CallFunction|Move))))

(event EventDamage
  (params (DamagePower :type Float%20%28double-precision%29))
  (Variables|Default|SetHealth (- (Variables|Default|GetHealth) DamagePower))
  (if (not (> (Variables|Default|GetHealth) 0.0))
    (CallFunction|Die)))

(fn ConstructionScript)

(fn Move
  (bind _random_distance (Variables|Default|GetRandom%20Distance))
  (LocalVariables|SetCurrentPos (Transformation|GetActorTransform))
  (Variables|/Script/Engine.MovementComponent|SetVelocity (Variables|Character|GetCharacterMovement) (Math|Vector|MakeVector 0.0 (* (Variables|Default|GetVelocity%20Y) (Variables|Default|Getleft)) 0.0))
  (if (or (> (.Y (Math|Vector|BreakVector (- (.location (LocalVariables|GetCurrentPos)) (.location (Variables|Default|GetStartDistance))))) _random_distance) (< (.Y (Math|Vector|BreakVector (- (.location (LocalVariables|GetCurrentPos)) (.location (Variables|Default|GetStartDistance))))) (* _random_distance -1.0)))
    (Variables|Default|SetisStoped true)
    (Variables|Default|Setleft (* (Variables|Default|Getleft) -1.0))))

(fn LookingforPlayer
  (bind _outhit (Collision|BoxTraceByChannel (Transformation|GetActorLocation) (Transformation|GetWorldLocation (Variables|Default|GetBox)) "0.000000,20.000000,20.000000" "0, 0, 0" "TraceTypeQuery1" false 0 "ForOneFrame"))
  (bind _asbp_first_person_character (Utilities|Casting|CastToBP_FirstPersonCharacter (.HitActor (Collision|BreakHitResult _outhit))))
  (CallFunction|Shooting _asbp_first_person_character))

(fn Shooting
  (params (Player :type BP%20First%20Person%20Character%20Object%20Reference))
  (bind _pointshoot (Variables|Default|GetPointShoot))
  (bind _returnvalue (Transformation|GetWorldTransform _pointshoot))
  (if (>= (Variables|Default|GetTime%20to%20Shoot) (Variables|Default|GetShooting%20Rate))
    (bind _returnvalue_2 (Game|SpawnActorfromClass "/Game/EHT01/Blueprints/BP_Projectile.BP_Projectile_C" (Math|Transform|MakeTransform (.location _returnvalue) (Math|Rotator|FindLookatRotation (.location _returnvalue) (.location (Transformation|GetActorTransform Player))) "1.000000,1.000000,1.000000") "Undefined" 0 0))
    (Variables|/Game/EHT01/Blueprints/BP_Projectile.BP_Projectile_C|SetDamagePower _returnvalue_2 25.0)
    (Variables|Default|SetTime%20to%20Shoot 0.0)))

(fn Die
  (Actor|DestroyActor))