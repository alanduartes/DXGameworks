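; BP_DummyBoy is an enemy that shoots at the first-person player, takes damage and destroys itself when health runs out.
; Each tick it box-traces toward its Box component and, if the player is hit, fires a BP_Projectile aimed at them, limited by ShootingRate.
; Tick also updates the widget health bar and turns it toward the player.
; Every Damage event triggers hit Niagara FX and adds to the player's score.
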(event EventBeginPlay
  (bind _asbp_first_person_character (Utilities|Casting|CastToBP_FirstPersonCharacter (Game|Player|GetPlayerPawn 0)))
  (Variables|Default|SetPlayer _asbp_first_person_character)
  (bind _aswgbp_enemy_helth_bar (Utilities|Casting|CastToWGBP_EnemyHelthBar (UserInterface|GetWidget (Variables|Default|GetHealthBarComponent))))
  (Variables|Default|SetAs%20WGBP%20Enemy%20Helth%20Bar _aswgbp_enemy_helth_bar))

(event EventTick
  (params (DeltaSeconds :type Float%20%28single-precision%29))
  ;[0.1864 0.3194 1] Tick
  (Variables|Default|SetTimeToShoot (+ DeltaSeconds (Variables|Default|GetTimeToShoot)))
  (CallFunction|LookingforPlayer)
  (CallFunction|HealthLookingtoCamera)
  (Progress|SetPercent (Variables|/Game/UI/WGBP_EnemyHelthBar.WGBP_EnemyHelthBar_C|GetHealthBar (Variables|Default|GetAs%20WGBP%20Enemy%20Helth%20Bar)) (/ (Variables|Default|GetHealth) 1e+02)))

(event EventDamage
  (params (DamagePower :type Float%20%28double-precision%29))
  (bind _player (Variables|Default|GetPlayer))
  ;[1 0.2983 0.368] Damage
  (Components|Activation|Activate (Variables|Default|GetHitNiagra_FX) true)
  (Variables|/Game/EHT01/Blueprints/BP_FirstPersonCharacter.BP_FirstPersonCharacter_C|SetScore _player (+ (Variables|/Game/EHT01/Blueprints/BP_FirstPersonCharacter.BP_FirstPersonCharacter_C|GetScore _player) (Variables|Default|GetPointsGive)))
  (bind _output_get (Variables|Default|SetHealth (- (Variables|Default|GetHealth) DamagePower)))
  (if (not (> _output_get 0.0))
    (CallFunction|Die)))

(fn ConstructionScript)

(fn Die
  (Actor|DestroyActor))

(fn LookingforPlayer
  (bind _returnvalue (Transformation|GetActorLocation))
  (bind (_x _y _z) (Class|KismetMathLibrary|BreakVector3f _returnvalue))
  (bind _outhit (Collision|BoxTraceByChannel (Math|Vector|MakeVector _x _y (+ _z 1e+02)) (Transformation|GetWorldLocation (Variables|Default|GetBox)) "20.000000,20.000000,50.000000" "0, 0, 0" "TraceTypeQuery1" false 0 "None"))
  (bind _asbp_first_person_character (Utilities|Casting|CastToBP_FirstPersonCharacter (.HitActor (Collision|BreakHitResult _outhit))))
  (CallFunction|Shooting _asbp_first_person_character))

(fn Shooting
  (params (Player :type BP%20First%20Person%20Character%20Object%20Reference))
  (bind _pointshoot (Variables|Default|GetPointShoot))
  (bind _returnvalue (Transformation|GetWorldTransform _pointshoot))
  (if (>= (Variables|Default|GetTimeToShoot) (Variables|Default|GetShootingRate))
    (bind _returnvalue_2 (Game|SpawnActorfromClass "/Game/EHT01/Blueprints/BP_Projectile.BP_Projectile_C" (Math|Transform|MakeTransform (.location _returnvalue) (Math|Rotator|FindLookatRotation (.location _returnvalue) (.location (Transformation|GetActorTransform Player))) "1.000000,1.000000,1.000000") "Undefined" 0 0))
    (Variables|/Game/EHT01/Blueprints/BP_Projectile.BP_Projectile_C|SetDamagePower _returnvalue_2 25.0)
    (Variables|Default|SetTimeToShoot 0.0)))

(fn HealthLookingtoCamera
  (bind _healthbarcomponent (Variables|Default|GetHealthBarComponent))
  (bind _returnvalue (Transformation|GetWorldLocation _healthbarcomponent))
  (Transformation|SetWorldTransform _healthbarcomponent (Math|Transform|MakeTransform _returnvalue (Math|Rotator|FindLookatRotation _returnvalue (Transformation|GetActorLocation (Variables|Default|GetPlayer))) "1.000000,1.000000,1.000000") false false))